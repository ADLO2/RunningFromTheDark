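; BP_Play_GameMode is the game mode for a play level, spawning players and starting the match with a countdown.
; It tracks connecting controllers and waits until their count matches the connected-player number stored in BP_GameInstance, while offline mode starts immediately with one player.
; Players spawn at player starts named by join index, then LevelStart triggers each controller's countdown and enables input three seconds later.
; Logouts remove controllers and decrement the expected count.
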(event Custom|LevelStart
  (Utilities|FlowControl|Delay 0.2)
  (for _array_element (Variables|Default|GetAll_ConnectedController)
    (Default|GameStartCountdown _array_element))
  (Utilities|FlowControl|Delay 3.0)
  (for _array_element_2 (Variables|Default|GetAll_ConnectedController)
    (Default|EnableAllInput _array_element_2)))

(event EventHandleStartingNewPlayer
  (params (NewPlayer :type Player%20Controller%20Object%20Reference))
  (bind _asbp_play_controller (Utilities|Casting|CastToBP_Play_Controller NewPlayer))
  (Utilities|Array|Add (Variables|Default|GetAll_ConnectedController) _asbp_play_controller)
  (bind _asbp_game_instance (Utilities|Casting|CastToBP_GameInstance (Game|GetGameInstance)))
  (Variables|Default|SetNumber_ExpectedPlayers (Variables|/Game/Gameplay/BP_GameInstance.BP_GameInstance_C|GetNumberOfConnectedPlayers _asbp_game_instance))
  (if (Variables|/Game/Gameplay/BP_GameInstance.BP_GameInstance_C|GetOffline _asbp_game_instance)
    (Variables|Default|SetNumber_ExpectedPlayers 1)
    (Class|GameModeBase|RestartPlayeratPlayerStart (Utilities|Array|Get(acopy) (Variables|Default|GetAll_ConnectedController)) (Class|GameModeBase|FindPlayerStart 0 "0"))
    (CallFunction|LevelStart)
    (elif (== (Variables|Default|GetNumber_ExpectedPlayers) (Utilities|Array|Length (Variables|Default|GetAll_ConnectedController)))
      (Utilities|FlowControl|Delay 0.5)
      (for (_array_element _array_index) (Variables|Default|GetAll_ConnectedController)
        (Class|GameModeBase|RestartPlayeratPlayerStart _array_element (Class|GameModeBase|FindPlayerStart _array_element (Utilities|String|ToString(Integer) _array_index))))
      (CallFunction|LevelStart))))

(event EventOnLogout
  (params (ExitingController :type Controller%20Object%20Reference))
  (bind _asbp_play_controller (Utilities|Casting|CastToBP_Play_Controller ExitingController))
  (Utilities|Array|RemoveItem (Variables|Default|GetAll_ConnectedController) _asbp_play_controller)
  (Math|Integer|DecrementInt (Variables|Default|GetNumber_ExpectedPlayers)))

(fn ConstructionScript)