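; BP_Play_Controller is the in-game player controller that sets up the HUD, input and player profile for a multiplayer session.
; On BeginPlay the local controller shows WB_IngameHUD, switches to game-only input and loads the saved profile, setting it directly on authority or sending it through a server event from a remote client.
; Further events re-enable pawn input, run the HUD start countdown, unhide the HUD and destroy the session to return to MenuMap.
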(event Custom|EnableAllInput
  (Input|EnableInput (Pawn|GetControlledPawn) self))

(event Custom|GameStartCountdown
  (Default|GameStartCountdown (Variables|Default|GetWB_IngameHUD)))

(event Custom|UnHide_IngameHUD
  (Widget|SetVisibility (Variables|Default|GetWB_IngameHUD) "Visible"))

(event Custom|EndClientSession
  (bind _asbp_game_instance (Utilities|Casting|CastToBP_GameInstance (Game|GetGameInstance)))
  (Variables|/Game/Gameplay/BP_GameInstance.BP_GameInstance_C|SetMP_isPauseMenuVisible _asbp_game_instance false)
  (|DestroySession self
    (:then
      (Game|OpenLevel(byName) "MenuMap"))))

(event Custom|Sever_SetPlayerProfile
  (params (S_PlayerProfile :type S%20Player%20Profile%20Structure))
  (Variables|Default|SetS_PlayerProfile S_PlayerProfile))

(event EventBeginPlay
  (if (Pawn|IsLocalPlayerController)
    (Viewport|RemoveAllWidgets)
    (CallFunction|UIShowIngameHUD)
    (Input|SetInputModeGameOnly self false)
    (Variables|Default|SetbShowMouseCursor false)
    (bind _returnvalue (SaveGame|LoadGamefromSlot "PlayerProfile_Slot"))
    (bind _assg_player_profile (Utilities|Casting|CastToSG_PlayerProfile _returnvalue))
    (Networking|SwitchHasAuthority
      (:Authority
        (Variables|Default|SetS_PlayerProfile (Variables|/Game/SaveData/SG_PlayerProfile.SG_PlayerProfile_C|GetPlayerProfile _assg_player_profile)))
      (:Remote
        (CallFunction|SeverSetPlayerProfile (Variables|/Game/SaveData/SG_PlayerProfile.SG_PlayerProfile_C|GetPlayerProfile _assg_player_profile))))))

(event EventTick
  (params (DeltaSeconds :type Float%20%28single-precision%29)))

(fn ConstructionScript)

(fn UIShowIngameHUD
  (Utilities|IsValid (Variables|Default|GetWB_IngameHUD)
    (:Is%20Valid
      _)
    (:Is%20Not%20Valid
      (bind _returnvalue (UserInterface|CreateWidget "/Game/Widget/WB_IngameHUD.WB_IngameHUD_C" self))
      (Variables|Default|SetWB_IngameHUD _returnvalue)))
  (UserInterface|Viewport|AddtoViewport (Variables|Default|GetWB_IngameHUD) 0)
  (return))