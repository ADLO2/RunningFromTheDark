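; Lobby menu game mode that tracks connected players and shows each one as a character in the lobby.
; Joining players on the lobby map get menu setup; on logout their character is destroyed and spot freed.
; Update events copy profiles into player states and refresh names, level selection and characters on each controller.
; Characters spawn at the first unused player spot, taking name, mesh and animation from profiles and a character data table.
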(event Custom|UpdateLobbyEvent
  (params (PlayerNames :type Boolean) (LevelSelection :type Boolean) (CharacterSelection :type Boolean))
  (Utilities|Array|Clear (Variables|Default|GetAll_PlayerProfile))
  (for (_array_element _array_index) (Variables|Default|GetAll_ConnectedPlayers)
    (Utilities|Array|SetArrayElem (Variables|Default|GetAll_PlayerProfile) _array_index (Variables|/Game/Gameplay/PB_MenuController.PB_MenuController_C|GetPlayer%20Profile _array_element) true)
    (bind _asbp_player_player_state (Utilities|Casting|CastToBP_Player_PlayerState (Variables|/Script/Engine.Controller|GetPlayerState _array_element)))
    (Variables|/Game/Gameplay/BP_Player_PlayerState.BP_Player_PlayerState_C|SetS_PlayerProfile _asbp_player_player_state (Variables|/Game/Gameplay/PB_MenuController.PB_MenuController_C|GetPlayer%20Profile _array_element)))
  (for (_array_element_2 _array_index_2) (Variables|Default|GetAll_ConnectedPlayers)
    (if PlayerNames
      (Default|UpdatePlayerNames _array_element_2 (Variables|Default|GetAll_PlayerProfile)))
    (if LevelSelection
      (Default|UpdateLevelSelection _array_element_2 (Variables|Default|GetSelectedLevelName)))
    (if CharacterSelection
      (CallFunction|UpdateSelectedCharacter _array_index_2))))

(event Custom|UpdateSelectedCharacter
  (params (PlayerIndex :type Integer))
  (bind _all_connectedplayers (Variables|Default|GetAll_ConnectedPlayers))
  (bind _all_playerprofile (Variables|Default|GetAll_PlayerProfile))
  (bind _output (Utilities|Array|Get(acopy) _all_connectedplayers PlayerIndex))
  (bind _output_2 (Utilities|Array|Get(acopy) _all_playerprofile PlayerIndex))
  (if (== (Variables|/Game/Gameplay/PB_MenuController.PB_MenuController_C|GetBP_LobbyCharacter (Utilities|Array|Get(acopy) (Variables|Default|GetAll_ConnectedPlayers) PlayerIndex)) 0)
    (bind _availplayerspot (CallFunction|GetLobbyPlayerSpot))
    (Variables|/Game/Gameplay/Lobby/BP_Lobby_PlayerSpot.BP_Lobby_PlayerSpot_C|SetIsUsed _availplayerspot true)
    (bind _returnvalue (Game|SpawnActorfromClass "/Game/Gameplay/Lobby/BP_LobbyCharacter.BP_LobbyCharacter_C" (Transformation|GetActorTransform _availplayerspot) "Undefined" "MultiplyWithRoot" 0 0))
    (Variables|/Game/Gameplay/PB_MenuController.PB_MenuController_C|SetBP_LobbyCharacter _output _returnvalue)
    (Variables|/Game/Gameplay/PB_MenuController.PB_MenuController_C|SetBP_LobbyPlayerSpot _output _availplayerspot))
  (Default|MCSetPlayerName (Variables|/Game/Gameplay/PB_MenuController.PB_MenuController_C|GetBP_LobbyCharacter (Utilities|Array|Get(acopy) (Variables|Default|GetAll_ConnectedPlayers) PlayerIndex)) (.playername _output_2))
  (bind _returnvalue_2 (Utilities|GetDataTableRow "/Game/Character/CharacterInfo_Table.CharacterInfo_Table" (.characterrowname _output_2))
    (:then
      (Default|MCSetCharMesh (Variables|/Game/Gameplay/PB_MenuController.PB_MenuController_C|GetBP_LobbyCharacter (Utilities|Array|Get(acopy) (Variables|Default|GetAll_ConnectedPlayers) PlayerIndex)) (.CharacterMesh (Utilities|Struct|BreakS_CharacterInfo _returnvalue_2)))
      (Default|MCPlayMeshAnimation (Variables|/Game/Gameplay/PB_MenuController.PB_MenuController_C|GetBP_LobbyCharacter (Utilities|Array|Get(acopy) (Variables|Default|GetAll_ConnectedPlayers) PlayerIndex)) (.LobbyAnimation (Utilities|Struct|BreakS_CharacterInfo _returnvalue_2))))))

(event Custom|UpdateCharacterForController
  (params (Controller :type PB%20Menu%20Controller%20Object%20Reference) (PlayerProfile :type S%20Player%20Profile%20Structure))
  (bind _all_connectedplayers (Variables|Default|GetAll_ConnectedPlayers))
  (bind _returnvalue (Utilities|Array|FindItem _all_connectedplayers Controller))
  (Utilities|Array|SetArrayElem (Variables|Default|GetAll_PlayerProfile) _returnvalue PlayerProfile true)
  (bind _asbp_player_player_state (Utilities|Casting|CastToBP_Player_PlayerState (Variables|/Script/Engine.Controller|GetPlayerState Controller)))
  (Variables|/Game/Gameplay/BP_Player_PlayerState.BP_Player_PlayerState_C|SetS_PlayerProfile _asbp_player_player_state PlayerProfile)
  (CallFunction|UpdateSelectedCharacter _returnvalue))

(event EventHandleStartingNewPlayer
  (params (NewPlayer :type Player%20Controller%20Object%20Reference))
  (bind _returnvalue (Game|GetCurrentLevelName true))
  (switch string _returnvalue
    (:LobbyMenuMap
      (bind _aspb_menu_controller (Utilities|Casting|CastToPB_MenuController NewPlayer))
      (Utilities|Array|Add (Variables|Default|GetAll_ConnectedPlayers) _aspb_menu_controller)
      (Default|CreateLobbyMenu _aspb_menu_controller)
      (Default|InitialSetup _aspb_menu_controller))))

(event EventOnLogout
  (params (ExitingController :type Controller%20Object%20Reference))
  (bind _aspb_menu_controller (Utilities|Casting|CastToPB_MenuController ExitingController))
  (if (== (Variables|/Game/Gameplay/PB_MenuController.PB_MenuController_C|GetBP_LobbyCharacter _aspb_menu_controller) 0)
    _
    (else
      (Actor|DestroyActor (Variables|/Game/Gameplay/PB_MenuController.PB_MenuController_C|GetBP_LobbyCharacter _aspb_menu_controller))
      (Variables|/Game/Gameplay/Lobby/BP_Lobby_PlayerSpot.BP_Lobby_PlayerSpot_C|SetIsUsed (Variables|/Game/Gameplay/PB_MenuController.PB_MenuController_C|GetBP_LobbyPlayerSpot _aspb_menu_controller) false)))
  (Utilities|Array|RemoveItem (Variables|Default|GetAll_ConnectedPlayers) _aspb_menu_controller)
  (CallFunction|UpdateLobbyEvent true false true))

(fn ConstructionScript)

(fn GetLobbyPlayerSpot
  (if (== (Utilities|Array|Length (Variables|Default|GetAll_LobbyPlayerSpotArray)) 0)
    (bind _outactors (Actor|GetAllActorsOfClass "/Game/Gameplay/Lobby/BP_Lobby_PlayerSpot.BP_Lobby_PlayerSpot_C"))
    (Variables|Default|SetAll_LobbyPlayerSpotArray _outactors))
  (bind _array_element (Utilities|Array|ForEachLoopwithBreak (Variables|Default|GetAll_LobbyPlayerSpotArray) :!label _label)
    (:LoopBody
      (if (not (Variables|/Game/Gameplay/Lobby/BP_Lobby_PlayerSpot.BP_Lobby_PlayerSpot_C|GetIsUsed _array_element))
        (goto _label Break)))
    (:Completed
      (return _array_element))))