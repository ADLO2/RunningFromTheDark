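; Playable second monster character, set to the "Mons2" row on its parent class, with crosshair dot and end-game widgets.
; Attack input runs a camera-forward sphere trace that applies damage, then plays a scream montage and sound through Sever/MC (server/multicast-named) events.
; A Holy Grenade hit, recognized by a damage value of exactly 99, disables local input and steps a camera post-process effect down over several seconds before restoring input.
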(event Custom|MC%20Damage
  (params (Damage :type Float%20%28double-precision%29))
  ;[1 1 1] Holy Grenade Hit
  (if (== Damage 99.0)
    (CallFunction|DisableAllInput (Pawn|GetLocalViewingPlayerController self))
    (Variables|/Script/Engine.CameraComponent|SetPostProcessSettings (Variables|Default|GetFollowCamera) (Utilities|Struct|MakePostProcessSettings 2.5e+03))
    (Utilities|FlowControl|Delay 3.0)
    (Variables|/Script/Engine.CameraComponent|SetPostProcessSettings (Variables|Default|GetFollowCamera) (Utilities|Struct|MakePostProcessSettings 1.5e+03))
    (Utilities|FlowControl|Delay 0.5)
    (Variables|/Script/Engine.CameraComponent|SetPostProcessSettings (Variables|Default|GetFollowCamera) (Utilities|Struct|MakePostProcessSettings 1e+03))
    (Utilities|FlowControl|Delay 0.5)
    (Variables|/Script/Engine.CameraComponent|SetPostProcessSettings (Variables|Default|GetFollowCamera) (Utilities|Struct|MakePostProcessSettings 5e+02))
    (Utilities|FlowControl|Delay 0.5)
    (Variables|/Script/Engine.CameraComponent|SetPostProcessSettings (Variables|Default|GetFollowCamera) (Utilities|Struct|MakePostProcessSettings 0.675))
    (Input|EnableInput (Pawn|GetLocalViewingPlayerController self))))

(event Custom|EndGame
  (bind _returnvalue (Game|GetPlayerController 0))
  ;[1 1 1] Start + End
  (bind _returnvalue_2 (UserInterface|CreateWidget "/Game/Widget/WB_Monster_EndGame.WB_Monster_EndGame_C"))
  (UserInterface|Viewport|AddtoViewport _returnvalue_2 0)
  (Variables|/Script/Engine.PlayerController|SetbShowMouseCursor _returnvalue true)
  (Input|SetInputModeUIOnly _returnvalue _returnvalue_2 "DoNotLock" false))

(event Custom|Sever_Attack
  ;[1 1 1] Screaming
  (CallFunction|MCAttack))

(event Custom|Sever_BehaviorAnim
  ;[1 1 1] Screaming
  (Utilities|FlowControl|Sequence
    (:then_0
      (CallFunction|MCPlayScream))
    (:then_1
      (CallFunction|MCPlayScreamSound))))

(event Custom|MC_Attack
  ;[1 1 1] Screaming
  (Variables|Default|SetIsAttacking true)
  (Variables|Default|SetIsAttackButtonPress true)
  (CallFunction|SeverAttackTrace)
  (CallFunction|SeverBehaviorAnim)
  (Variables|Default|SetIsAttacking false)
  (Variables|Default|SetIsAttackButtonPress false))

(event Custom|CreateWidget
  ;[1 1 1] Start + End
  (bind _returnvalue (UserInterface|CreateWidget "/Game/Widget/WB_Dot.WB_Dot_C" (Game|GetPlayerController 0)))
  (UserInterface|Viewport|AddtoViewport _returnvalue 0))

(event Custom|MC_PlayScream
  ;[1 1 1] Screaming
  (Animation|Montage|PlayMontage (Variables|Character|GetMesh) "/Game/Character/Monster/2/Animation/Zombie2_Scream_Montage.Zombie2_Scream_Montage"))

(event Custom|MC_PlayScreamSound
  ;[1 1 1] Screaming
  (Audio|PlaySoundatLocation "/Game/Sound/MONSTER_SCREAM_______.MONSTER_SCREAM_______" (Transformation|GetWorldLocation (Variables|Default|GetSocketLocation)) "0, 0, 0" 0.5 1.0 0.0 0 0 0 0))

(event EventBeginPlay
  ;[1 1 1] Start + End
  (CallFunction|CreateWidget))

(event Game|Damage|EventAnyDamage
  (params (Damage :type Float%20%28single-precision%29) (DamageType :type Damage%20Type%20Object%20Reference) (InstigatedBy :type Controller%20Object%20Reference) (DamageCauser :type Actor%20Object%20Reference))
  ;[1 1 1] Holy Grenade Hit
  (CallFunction|MCDamage Damage))

(event Input|ActionEvents|InputActionAttack
  (params (Key :type Key%20Structure :default "None"))
  ;[1 1 1] Screaming
  (:Pressed
    (if (not (Variables|Default|GetIsAttacking))
      (CallFunction|SeverAttack))))

(fn ConstructionScript
  (Variables|Default|SetCharacterRowName "Mons2")
  (|CallParentFunction))

(fn SeverAttackTrace
  (bind _followcamera (Variables|Default|GetFollowCamera))
  (bind _returnvalue (Transformation|GetWorldTransform _followcamera))
  (bind _outhit (Collision|SphereTraceByChannel (.location _returnvalue) (+ (.location _returnvalue) (* (Math|Vector|GetForwardVector (.rotation _returnvalue)) 10000)) 6e+01 "TraceTypeQuery2" false 0 "ForDuration"))
  (Game|Damage|ApplyDamage (.hitactor _outhit) 1.0 0 0)
  (return))