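; BP_Things is an item that a Survivor picks up on interaction and that can later be dropped.
; It starts Dropped, with a physics-simulated skeletal mesh and an overlap sphere, and shows a "Pick Up" prompt attached to the mesh.
; SetItemState switches to Equipped on pickup, disabling physics and collision and resetting the mesh's relative transform, while Drop restores the Dropped state.
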(event EventBeginPlay
  (Private|SetItemState "NewEnumerator0"))

(event EventOnInteracted
  (params (Survivor :type BP%20Survivor%20Object%20Reference))
  (Default|PickUp Survivor self)
  (Private|SetItemState "NewEnumerator1"))

(fn ConstructionScript
  (|CallParentFunction))

(fn GetInteractionText
  (return "Pick Up"))

(fn GetInterationTextAttach
  (return (Variables|Default|GetSkeletalMesh)))

(fn SetItemState
  (params (NewItemState :type E_ItemState%20Enum :default "NewEnumerator0"))
  (bind _skeletalmesh (Variables|Default|GetSkeletalMesh))
  (bind _skeletalmesh_2 (Variables|Default|GetSkeletalMesh))
  (bind _output_get (Variables|Private|SetItemState NewItemState))
  (switch Utilities|FlowControl|Switch|SwitchonE_ItemState _output_get
    (:NewEnumerator0
      (Collision|SetCollisionProfileName (Variables|Default|GetSphere) "OverlapAllDynamic" true :!class /Script/Engine.PrimitiveComponent)
      (Physics|SetSimulatePhysics _skeletalmesh_2 true)
      (Collision|SetCollisionProfileName _skeletalmesh_2 "DroppedItem" true :!class /Script/Engine.PrimitiveComponent))
    (:NewEnumerator1
      (Collision|SetCollisionProfileName (Variables|Default|GetSphere) "NoCollision" true :!class /Script/Engine.PrimitiveComponent)
      (Physics|SetSimulatePhysics _skeletalmesh false)
      (Collision|SetCollisionProfileName _skeletalmesh "NoCollision" true :!class /Script/Engine.PrimitiveComponent)
      (Transformation|ResetRelativeTransform (Variables|Default|GetSkeletalMesh)))))

(fn Drop
  (Private|SetItemState "NewEnumerator0"))